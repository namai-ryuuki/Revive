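; Origin marker actor that shows a beam from the ThirdPersonCharacter's FirstPosition to the player's current location.
; Each Tick it draws a debug trace along that line, aims the Beam and scales it uniformly by distance.
; When the character raises CreateOriginBP and FirstPosition has changed, it clears the flag, spawns a new Origin_BP there and destroys itself.
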(event EventTick
  (params (DeltaSeconds :type Float%20%28single-precision%29))
  (bind _returnvalue (Game|Player|GetPlayerPawn 0))
  (bind _returnvalue_2 (Game|Player|GetPlayerPawn 0))
  (bind _beam (Variables|Default|GetBeam))
  (bind _returnvalue_3 (Transformation|GetActorLocation _returnvalue))
  (bind _asthird_person_character (Utilities|Casting|CastToThirdPersonCharacter _returnvalue))
  (bind _asthird_person_character_2 (Utilities|Casting|CastToThirdPersonCharacter _returnvalue_2))
  (bind _firstposition (Variables|/Game/Revive/Blueprints/Character/ThirdPersonCharacter.ThirdPersonCharacter_C|GetFirstPosition _asthird_person_character))
  (bind _firstposition_2 (Variables|/Game/Revive/Blueprints/Character/ThirdPersonCharacter.ThirdPersonCharacter_C|GetFirstPosition _asthird_person_character_2))
  ;[1 1 1] 吸ったり与えたりしたとき原点移動時、そこから線伸ばしてエフェクト付ける
  (Utilities|FlowControl|Sequence
    (:then_0
      (Collision|LineTraceByChannel _firstposition _returnvalue_3 "TraceTypeQuery1" false 0 "ForOneFrame" true "(R=1.000000,G=0.000000,B=0.000000,A=1.000000)" "(R=1.000000,G=0.036275,B=0.000000,A=1.000000)")
      (Transformation|SetWorldRotation _beam (Math|Rotator|FindLookatRotation _firstposition _returnvalue_3) false false)
      (Transformation|SetRelativeScale3D _beam (Math|Conversions|ToVector(Float) (/ (Math|Vector|VectorLength (- _returnvalue_3 _firstposition)) 2e+02))))
    (:then_1
      (if (Variables|/Game/Revive/Blueprints/Character/ThirdPersonCharacter.ThirdPersonCharacter_C|GetCreate_OriginBP _asthird_person_character_2)
        (if (not (Class|KismetMathLibrary|EqualExactlyVectorVector (Variables|Default|GetFPos_vs_Vector) _firstposition_2))
          (Variables|Default|SetFPos_vs_Vector _firstposition_2)
          (Variables|/Game/Revive/Blueprints/Character/ThirdPersonCharacter.ThirdPersonCharacter_C|SetCreate_OriginBP _asthird_person_character_2 false)
          (Game|SpawnActorfromClass "Origin_BP_C" (Math|Conversions|ToTransform(Vector) _firstposition_2) "Undefined" 0 0)
          (Actor|DestroyActor))))))

(event EventBeginPlay
  (Variables|Default|SetFPos_vs_Vector (Variables|/Game/Revive/Blueprints/Character/ThirdPersonCharacter.ThirdPersonCharacter_C|GetFirstPosition (.AsThird%20Person%20Character (Utilities|Casting|CastToThirdPersonCharacter (Game|Player|GetPlayerPawn 0)))))
  (Variables|/Game/Revive/Blueprints/Character/ThirdPersonCharacter.ThirdPersonCharacter_C|SetCreate_OriginBP (.AsThird%20Person%20Character (Utilities|Casting|CastToThirdPersonCharacter (Game|Player|GetPlayerPawn 0))) false))

(fn ConstructionScript)