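; Fire planet (Wakusei) that sets normal and energy planets within its reach burning.
; Sphere overlap events manage fire-hit flags on those planets, while Tick scales the Bakuha blast range with PHP.
; Each Tick scans all planets and ignites flagged ones, overriding ice only where its PHP exceeds an ice planet's.
; It keeps its own IceFlag cleared and sets an ice-planet tick prerequisite at BeginPlay.
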(event OnComponentEndOverlap(Sphere)
  (params (OverlappedComponent :type Primitive%20Component%20Object%20Reference) (OtherActor :type Actor%20Object%20Reference) (OtherComp :type Primitive%20Component%20Object%20Reference) (OtherBodyIndex :type Integer))
  ;[1 1 1] 貴様（☆）をもやす
  (Utilities|FlowControl|Sequence
    (:then_0
      ;;[1 1 1] 通常惑星用（sphereに親クラスwakuseiと当たっていなかったらFIREHITをFALSE
      (if (Utilities|ClassIsChildOf (Utilities|GetClass OtherActor) "/Game/Revive/Blueprints/MapObject/Wakusei_Blueprint.Wakusei_Blueprint_C")
        (bind _aswakusei_blueprint (Utilities|Casting|CastToWakusei_Blueprint OtherActor))
        (if (Class|PrimitiveComponent|IsOverlappingComponent (Variables|Default|GetSphere) (Variables|/Game/Revive/Blueprints/MapObject/Wakusei_Blueprint.Wakusei_Blueprint_C|GetSphere _aswakusei_blueprint))
          (Variables|/Game/Revive/Blueprints/MapObject/Wakusei_Blueprint.Wakusei_Blueprint_C|SetFireHit _aswakusei_blueprint false))))
    (:then_1
      ;;[1 1 1] エネルギー惑星用（sphereに親クラスwakuseiと当たっていなかったらFIREHITをFALSE
      (if (Utilities|ClassIsChildOf (Utilities|GetClass OtherActor) "/Game/Revive/Blueprints/MapObject/EnergieWakusei_Blueprint.EnergieWakusei_Blueprint_C")
        (bind _asenergie_wakusei_blueprint (Utilities|Casting|CastToEnergieWakusei_Blueprint OtherActor))
        (if (Class|PrimitiveComponent|IsOverlappingComponent (Variables|Default|GetSphere) (Variables|/Game/Revive/Blueprints/MapObject/EnergieWakusei_Blueprint.EnergieWakusei_Blueprint_C|GetSphere _asenergie_wakusei_blueprint))
          (Variables|/Game/Revive/Blueprints/MapObject/EnergieWakusei_Blueprint.EnergieWakusei_Blueprint_C|SetFireEHit _asenergie_wakusei_blueprint false))))))

(event OnComponentBeginOverlap(Sphere)
  (params (OverlappedComponent :type Primitive%20Component%20Object%20Reference) (OtherActor :type Actor%20Object%20Reference) (OtherComp :type Primitive%20Component%20Object%20Reference) (OtherBodyIndex :type Integer) (bFromSweep :type Boolean) (SweepResult :type Hit%20Result%20Structure%20%28by%20ref%29))
  ;[1 1 1] 貴様（☆）をもやす
  (Utilities|FlowControl|Sequence
    (:then_0
      ;;[1 1 1] 通常惑星用（sphereに親クラスwakuseiと当たったらFIREHITをTRUE）
      (if (Utilities|ClassIsChildOf (Utilities|GetClass OtherActor) "/Game/Revive/Blueprints/MapObject/Wakusei_Blueprint.Wakusei_Blueprint_C")
        (bind _aswakusei_blueprint (Utilities|Casting|CastToWakusei_Blueprint OtherActor))
        (if (Class|PrimitiveComponent|IsOverlappingComponent (Variables|Default|GetSphere) (Variables|/Game/Revive/Blueprints/MapObject/Wakusei_Blueprint.Wakusei_Blueprint_C|GetSphere _aswakusei_blueprint))
          (Variables|/Game/Revive/Blueprints/MapObject/Wakusei_Blueprint.Wakusei_Blueprint_C|SetFireHit _aswakusei_blueprint true))))
    (:then_1
      ;;[1 1 1] エネルギー惑星用（sphereにEnergiewakuseiと当たったらFIREEHITをTRUE）
      (if (Utilities|ClassIsChildOf (Utilities|GetClass OtherActor) "/Game/Revive/Blueprints/MapObject/EnergieWakusei_Blueprint.EnergieWakusei_Blueprint_C")
        (bind _asenergie_wakusei_blueprint (Utilities|Casting|CastToEnergieWakusei_Blueprint OtherActor))
        (if (Class|PrimitiveComponent|IsOverlappingComponent (Variables|Default|GetSphere) (Variables|/Game/Revive/Blueprints/MapObject/EnergieWakusei_Blueprint.EnergieWakusei_Blueprint_C|GetSphere _asenergie_wakusei_blueprint))
          (Variables|/Game/Revive/Blueprints/MapObject/EnergieWakusei_Blueprint.EnergieWakusei_Blueprint_C|SetFireEHit _asenergie_wakusei_blueprint true))))))

(event EventBeginPlay
  (|CallParentFunction)
  (Utilities|IsValid "/Game/Revive/Blueprints/MapObject/Wakusei_Child_Ice_BP.Wakusei_Child_Ice_BP"
    (:Is%20Valid
      (Actor|Tick|AddTickPrerequisiteActor 0))))

(event Collision|EventActorBeginOverlap
  (params (OtherActor :type Actor%20Object%20Reference))
  (|CallParentFunction OtherActor) ; This node is disabled and will not be called.\nDrag off pins to build functionality.
)

(event EventTick
  (params (DeltaSeconds :type Float%20%28single-precision%29))
  (|CallParentFunction DeltaSeconds)
  (Utilities|FlowControl|Sequence
    (:then_0
      (bind _output_get (Variables|Default|SetBakuhaHanni (Math|Conversions|ToVector(Float) (* (Variables|Default|GetP_HP) 0.5))))
      (Transformation|SetWorldScale3D (Variables|Default|Getbakuha) _output_get))
    (:then_1
      ;[1 1 1] 惑星をもやす処理
      (bind _outactors (Actor|GetAllActorsOfClass "/Game/Revive/Blueprints/MapObject/Wakusei_Blueprint.Wakusei_Blueprint_C"))
      (for _array_element _outactors
        (if (Variables|/Game/Revive/Blueprints/MapObject/Wakusei_Blueprint.Wakusei_Blueprint_C|GetFireHit _array_element)
          (if (Variables|/Game/Revive/Blueprints/MapObject/Wakusei_Blueprint.Wakusei_Blueprint_C|GetIceHit _array_element)
            (bind _outactors_2 (Actor|GetAllActorsOfClass "/Game/Revive/Blueprints/MapObject/Wakusei_Child_Ice_BP.Wakusei_Child_Ice_BP_C"))
            (for _array_element_2 _outactors_2
              (if (< (Variables|/Game/Revive/Blueprints/MapObject/Wakusei_Blueprint.Wakusei_Blueprint_C|GetP_HP _array_element_2) (Variables|Default|GetP_HP))
                (Default|FireBPIF _array_element true)
                (Default|ICEBPIF _array_element false)))
            (else
              (Default|FireBPIF _array_element true)
              (Default|ICEBPIF _array_element false))))))
    (:then_2
      ;[1 1 1] エネルギー惑星をもやす処理
      (bind _outactors_3 (Actor|GetAllActorsOfClass "/Game/Revive/Blueprints/MapObject/EnergieWakusei_Blueprint.EnergieWakusei_Blueprint_C"))
      (for _array_element_3 _outactors_3
        (if (Variables|/Game/Revive/Blueprints/MapObject/EnergieWakusei_Blueprint.EnergieWakusei_Blueprint_C|GetFireEHit _array_element_3)
          (if (Variables|/Game/Revive/Blueprints/MapObject/EnergieWakusei_Blueprint.EnergieWakusei_Blueprint_C|GetIceHit _array_element_3)
            (bind _outactors_4 (Actor|GetAllActorsOfClass "/Game/Revive/Blueprints/MapObject/Wakusei_Child_Ice_BP.Wakusei_Child_Ice_BP_C"))
            (for _array_element_4 _outactors_4
              (if (< (Variables|/Game/Revive/Blueprints/MapObject/Wakusei_Blueprint.Wakusei_Blueprint_C|GetP_HP _array_element_4) (Variables|Default|GetP_HP))
                (Default|FireBPIF _array_element_3 true)
                (Default|ICEBPIF _array_element_3 false)))
            (else
              (Default|FireBPIF _array_element_3 true)
              (Default|ICEBPIF _array_element_3 false))))))
    (:then_3
      (Variables|Default|SetIceFlag false))))

(event EventICEBPIF
  (params (flag :type Boolean))
  (Variables|Default|SetIceFlag false))

(fn ConstructionScript)