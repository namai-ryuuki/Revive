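; Tree planet map object, apparently a child of a planet Blueprint, whose attached vine (Tuta_BP child actor) shrinks as the planet's HP is absorbed.
; Each Tick it scales the vine and its collision box along Y by the absolute HP ratio and offsets the vine in Y by current HP.
; At 5% HP or less both are scaled to zero, while the planet mesh, HP component and spheres keep fixed scales.
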(event EventBeginPlay
  (|CallParentFunction)
  (Transformation|SetWorldScale3D (Variables|Default|GetStaticMeshComponent) "3.000000,3.000000,3.000000") ; 大きさが3以上だったら３にする
)

(event Collision|EventActorBeginOverlap
  (params (OtherActor :type Actor%20Object%20Reference))
  (|CallParentFunction OtherActor) ; This node is disabled and will not be called.\nDrag off pins to build functionality.
)

(event EventTick
  (params (DeltaSeconds :type Float%20%28single-precision%29))
  (|CallParentFunction DeltaSeconds)
  (Utilities|FlowControl|Sequence
    (:then_0
      (CallFunction|NewFunction0))))

(fn ConstructionScript
  (|CallParentFunction))

(fn NewFunction0
  (bind _childactor (Variables|Default|GetChildActor))
  (bind _childactor_2 (Variables|Default|GetChildActor))
  (bind _p_hp (Variables|Default|GetP_HP))
  (bind _staticmeshcomponent (Variables|Default|GetStaticMeshComponent))
  (bind _p_maxhp (Variables|Default|GetP_MAXHP))
  (bind _returnvalue (Transformation|GetWorldLocation _staticmeshcomponent))
  (bind _returnvalue_2 (/ _p_hp _p_maxhp))
  (bind _childactor_3 (Variables|/Script/Engine.ChildActorComponent|GetChildActor _childactor))
  (bind _returnvalue_3 (Math|Float|Absolute(Float) _returnvalue_2))
  (bind _returnvalue_4 (Math|Conversions|ToVector(Float) _returnvalue_3))
  (bind _returnvalue_5 (* (.y _returnvalue_4) 5.0))
  ;[1 1 1] 当たり判定の大きさ
  (Transformation|SetWorldScale3D (Variables|Default|GetStaticMeshComponent) "3.000000,3.000000,3.000000") ; 星の大きさは固定
  (bind _output_get (Variables|Default|Setscale_float _returnvalue_3))
  (if (<= _output_get 0.05) ; HPが５％以下ならツタ表示しない
    (Transformation|SetWorldScale3D (Variables|/Game/Revive/Blueprints/MapObject/Tuta_BP.Tuta_BP_C|GetBox (.AsTuta%20BP (Utilities|Casting|CastToTuta_BP (Variables|/Script/Engine.ChildActorComponent|GetChildActor _childactor_2)))) "0, 0, 0")
    (Transformation|SetWorldScale3D _childactor_2 "0, 0, 0")
    (else
      (Transformation|SetWorldScale3D (Variables|/Game/Revive/Blueprints/MapObject/Tuta_BP.Tuta_BP_C|GetBox (.AsTuta%20BP (Utilities|Casting|CastToTuta_BP _childactor_3))) (Math|Vector|MakeVector 0.5 _returnvalue_5 0.5))
      (Transformation|SetWorldScale3D _childactor (Math|Vector|MakeVector 0.5 _returnvalue_5 0.5))
      (Transformation|SetActorLocation _childactor_3 (Math|Vector|MakeVector (.x _returnvalue) (+ (.y _returnvalue) (* (Variables|Default|GetP_HP) 5.0)) (.z _returnvalue)) false false)))
  (Transformation|SetWorldScale3D (Variables|Default|GetHP) "2.500000,2.500000,2.500000")
  (Transformation|SetWorldScale3D (Variables|Default|GetSphere) "8.000000,8.000000,8.000000")
  (Transformation|SetWorldScale3D (Variables|Default|GetSphere1) "7.000000,8.000000,8.000000"))