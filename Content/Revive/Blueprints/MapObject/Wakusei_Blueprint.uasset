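; Planet (Wakusei) actor whose HP the player drains by absorbing or refills by giving energy.
; Hit and overlap flags gate the HP events; the sphere overlap also notifies the player and breakable walls.
; Tick scales the mesh with HP up to a cap, updates camera-facing HP widgets, toggles proximity particles and shows blast range on player hold.
; Inside an axis range, it circles its start position until the player comes near.
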(event OnComponentBeginOverlap(Sphere)
  (params (OverlappedComponent :type Primitive%20Component%20Object%20Reference) (OtherActor :type Actor%20Object%20Reference) (OtherComp :type Primitive%20Component%20Object%20Reference) (OtherBodyIndex :type Integer) (bFromSweep :type Boolean) (SweepResult :type Hit%20Result%20Structure%20%28by%20ref%29))
  ;[1 1 1] プレイヤーとの当たり判定（放出・吸収用）
  (Utilities|FlowControl|Sequence
    (:then_0
      (if (== (Utilities|GetClass OtherActor) "/Game/Revive/Blueprints/Character/ThirdPersonCharacter.ThirdPersonCharacter_C")
        (Class|HITBPIF|HitCall(Message) OtherActor true)
        (if (not (Variables|Default|GetPlayer_In))
          (Variables|Default|SetPlayer_In true)
          (if (>= (Variables|Default|GetP_HP) 1e+01)
            (Variables|Default|SetP_TIMEHP (Variables|Default|GetP_HP))))))
    (:then_1
      (if (== (Utilities|GetClass OtherActor) "/Game/Revive/Blueprints/MapObject/BreakWall_BP.BreakWall_BP_C")
        (Class|HITBPIF|HitCall(Message) OtherActor true)))))

(event OnComponentEndOverlap(Sphere)
  (params (OverlappedComponent :type Primitive%20Component%20Object%20Reference) (OtherActor :type Actor%20Object%20Reference) (OtherComp :type Primitive%20Component%20Object%20Reference) (OtherBodyIndex :type Integer))
  ;[1 1 1] プレイヤーとの当たり判定（放出・吸収用）
  (if (== (Utilities|GetClass OtherActor) "/Game/Revive/Blueprints/Character/ThirdPersonCharacter.ThirdPersonCharacter_C")
    (Class|HITBPIF|HitCall(Message) OtherActor false)
    (Variables|Default|SetPlayer_In false)))

(event EventBeginPlay
  (bind _p_hp (Variables|Default|GetP_HP))
  ;[1 1 1] BeginPlay
  (bind _ashp_ui (Utilities|Casting|CastToHP_UI (UserInterface|GetUserWidgetObject (Variables|Default|GetHP))))
  (bind _output_get (Variables|Default|SetHP_UI _ashp_ui))
  (Variables|/Game/Revive/Blueprints/UI/HP_UI.HP_UI_C|SetHP _output_get 1.0)
  (bind _ashp_visible_ui (Utilities|Casting|CastToHP_Visible_UI (UserInterface|GetUserWidgetObject (Variables|Default|GetHP_Visibli))))
  (bind _output_get_2 (Variables|Default|SetHP_NUMBER _ashp_visible_ui))
  (Variables|/Game/Revive/Blueprints/UI/HP_Visible_UI.HP_Visible_UI_C|SetHP _output_get_2 _p_hp)
  (Variables|Default|SetP_TIME_MAXHP _p_hp)
  (Components|Activation|Deactivate (Variables|Default|GetParticleSystem)) ; パーティクル停止
  (Components|Activation|Deactivate (Variables|Default|GetParticleSystem1)) ; パーティクル停止
  (Variables|Default|SetStartPosition (Transformation|GetActorLocation))
  (Variables|Default|SetP_TIMEHP (Variables|Default|GetP_HP)))

(event EventTick
  (params (DeltaSeconds :type Float%20%28single-precision%29))
  (bind _staticmeshcomponent (Variables|Debug|GetStaticMeshComponent))
  (bind _p_hp (Variables|Default|GetP_HP))
  (bind _bakuha (Variables|Default|Getbakuha))
  (bind _returnvalue (* _p_hp 0.07))
  (bind _returnvalue_2 (Math|Float|Absolute(Float) _returnvalue))
  (bind _returnvalue_3 (Math|Conversions|ToVector(Float) _returnvalue_2))
  ;[1 1 1 1 36] Tick
  (Utilities|FlowControl|Sequence
    (:then_0
      ;;[1 1 1] HPゲージが常にカメラを向くように設定
      (|CameraMove))
    (:then_1
      ;;[1 1 1] HPの割合を求める
      (|HP＿WARIAI))
    (:then_2
      ;;[1 1 1] パーティクルON/OFF
      (|Particle))
    (:then_3
      ;;[1 1 1] 当たり判定の大きさ
      (if (> (Variables|Default|GetP_HP) 0.0)
        (bind _output_get (Variables|Default|Setscale_float _returnvalue_2))
        (if (>= _output_get 3.0)
          (Transformation|SetWorldScale3D _staticmeshcomponent "3.000000,3.000000,3.000000") ; 大きさが3以上だったら３にする
          (else
            (Transformation|SetWorldScale3D _staticmeshcomponent _returnvalue_3)))
        (Development|PrintString (Utilities|String|ToString(Vector) _returnvalue_3) true true "(R=0.744709,G=1.000000,B=0.000000,A=1.000000)" 0.0)
        ;;;[1 1 1] コリジョン大きさ変更
        (Transformation|SetWorldScale3D (Variables|Default|GetSphere) "10.000000,10.000000,10.000000")
        (Transformation|SetWorldScale3D (Variables|Default|GetSphere1) "7.000000,8.000000,8.000000")
        (Transformation|SetWorldScale3D (Variables|Default|Getbakuha) (Variables|Default|GetBakuhaHanni))
        (Transformation|SetWorldScale3D (Variables|Default|GetHP) "2.500000,2.500000,2.500000")))
    (:then_4
      (Utilities|FlowControl|Sequence
        (:then_0
          ;;[1 1 1] 爆破範囲可視化
          (if (Variables|/Game/Revive/Blueprints/Character/ThirdPersonCharacter.ThirdPersonCharacter_C|Getbakuhacheck_hold (.AsThird%20Person%20Character (Utilities|Casting|CastToThirdPersonCharacter (Game|GetPlayerCharacter 0))))
            (Development|SetHiddeninGame _bakuha false false)
            (else
              (Development|SetHiddeninGame _bakuha true false))))
        (:then_1
          ;;[1 1 1] 軸の範囲に入ったら星の回転
          (if (Math|Boolean|NotEqual(Boolean) (Variables|Default|GetPlayer_In) true) ; プレイヤーに接触してたら止まる
            (if (Variables|Default|GetZiku_In)
              (Transformation|AddActorLocalRotation (Variables|Default|GetRotationStarSpeed) false false)
              (bind _output_get_2 (Variables|Default|SetDirectionVector (Math|Rotator|GetRotationXVector (Transformation|GetActorRotation))))
              (Transformation|SetActorLocation (+ (Variables|Default|GetStartPosition) (* (Math|Vector|Normalize _output_get_2) (Variables|Default|GetDistance))) false false))))))
    (:then_5
      (Development|PrintString (Utilities|String|ToString(Boolean) (Variables|Default|Getplayer_hit)) true true "(R=0.000000,G=0.660000,B=1.000000,A=1.000000)" 0.0))))

(event EventWakuseiHpDown
  ;[1 1 1] 吸い込まれたときの処理
  (if (Variables|Default|Getplayer_hit)
    (bind _output_get (Variables|Default|SetP_HP (- (Variables|Default|GetP_HP) (Variables|Default|Gethp_add))))
    (Variables|Default|SetP_TIME_MAXHP _output_get)))

(event EventZikuHanni
  (params (flag :type Boolean) (location :type Vector :default "0, 0, 0") (Component :type Static%20Mesh%20Component%20Object%20Reference))
  ;[1 1 1] 回転する軸に入ってたらtrue
  (Variables|Default|SetZiku_In flag)
  (Variables|Default|SetRotationMove location))

(event Collision|EventActorBeginOverlap
  (params (OtherActor :type Actor%20Object%20Reference)))

(event EventLimeHit
  (params (flag :type Boolean))
  (Variables|Default|Setplayer_hit flag))

(event EventWakuseiHpAdd
  ;[1 1 1] エネルギーを与えられたときの処理
  (if (Variables|Default|Getplayer_hit)
    (if (Variables|Default|GetPlayer_In)
      (if (>= (Variables|Default|GetP_MAXHP) (Variables|Default|GetP_HP))
        (bind _output_get (Variables|Default|SetP_HP (+ (Variables|Default|GetP_HP) (Variables|Default|Gethp_add))))
        (Variables|Default|SetP_TIME_MAXHP _output_get)
        (bind _asthird_person_character (Utilities|Casting|CastToThirdPersonCharacter (Game|GetPlayerCharacter 0)))
        (Default|HPMINUSOK _asthird_person_character)))))

(fn ConstructionScript
  (bind _p_maxhp (Variables|Default|GetP_MAXHP))
  (bind _staticmeshcomponent (Variables|Debug|GetStaticMeshComponent))
  (bind _returnvalue (* _p_maxhp 0.07))
  (bind _returnvalue_2 (Math|Float|Absolute(Float) _returnvalue))
  (Transformation|SetWorldScale3D (Variables|Default|Getbakuha) (Variables|Default|GetBakuhaHanni))
  (bind _output_get (Variables|Default|Setscale_float _returnvalue_2))
  (if (>= _output_get 3.0)
    (Transformation|SetWorldScale3D _staticmeshcomponent "3.000000,3.000000,3.000000") ; 大きさが3以上だったら３にする
    (else
      (Transformation|SetWorldScale3D _staticmeshcomponent (Math|Conversions|ToVector(Float) _returnvalue_2))))
  (Transformation|SetWorldScale3D (Variables|Default|GetSphere) "10.000000,10.000000,10.000000")
  (Transformation|SetWorldScale3D (Variables|Default|GetSphere1) "7.000000,8.000000,8.000000")
  (Rendering|SetVisibility (Variables|Default|GetSphere1) false false))