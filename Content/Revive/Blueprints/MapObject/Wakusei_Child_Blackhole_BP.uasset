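; Planet Blueprint variant that turns into a black hole linked to a white hole once its HP reaches zero.
; BlackHoleCollision flags planets and the player for Tick-driven pull, with planets accelerating inward along a flattened vector cached on overlap.
; WarpCollision teleports planets to the white hole, which pushes them out with decreasing speed until outside WHRadius.
; The player instead glides there with a hidden mesh until the character's WarpFlag clears.
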(event OnComponentEndOverlap(BlackHoleCollision)
  (params (OverlappedComponent :type Primitive%20Component%20Object%20Reference) (OtherActor :type Actor%20Object%20Reference) (OtherComp :type Primitive%20Component%20Object%20Reference) (OtherBodyIndex :type Integer))
  ;[1 1 1] BHとの当たり判定
  (if (Variables|Default|GetBHWHFlag)
    (bind _outactors (Actor|GetAllActorsOfClass "/Game/Revive/Blueprints/Character/ThirdPersonCharacter.ThirdPersonCharacter_C"))
    (for _array_element _outactors
      (if (== _array_element OtherActor)
        (Variables|Default|SetBHPlayerSuikomiFlag false)))))

(event OnComponentBeginOverlap(BlackHoleCollision)
  (params (OverlappedComponent :type Primitive%20Component%20Object%20Reference) (OtherActor :type Actor%20Object%20Reference) (OtherComp :type Primitive%20Component%20Object%20Reference) (OtherBodyIndex :type Integer) (bFromSweep :type Boolean) (SweepResult :type Hit%20Result%20Structure%20%28by%20ref%29))
  ;[1 1 1] BHとの当たり判定
  (if (Variables|Default|GetBHWHFlag)
    _
    (else
      _))
  (bind _outactors (Actor|GetAllActorsOfClass "Wakusei_Child_Blackhole_BP_C"))
  (for _array_element _outactors
    (if (not (== _array_element OtherActor)) ; BHをはじく
      (if (Utilities|ClassIsChildOf (Utilities|GetClass OtherActor) "/Game/Revive/Blueprints/MapObject/Wakusei_Blueprint.Wakusei_Blueprint_C") ; 惑星かどうか
        (bind _aswakusei_blueprint (Utilities|Casting|CastToWakusei_Blueprint OtherActor))
        (if (Class|PrimitiveComponent|IsOverlappingComponent (Variables|Default|GetBlackHoleCollision) (Variables|/Game/Revive/Blueprints/MapObject/Wakusei_Blueprint.Wakusei_Blueprint_C|GetSphere _aswakusei_blueprint))
          (Variables|/Game/Revive/Blueprints/MapObject/Wakusei_Blueprint.Wakusei_Blueprint_C|SetBlackHoleFlag _aswakusei_blueprint true)
          (bind _output_get (Variables|/Game/Revive/Blueprints/MapObject/Wakusei_Blueprint.Wakusei_Blueprint_C|SetBHMove _aswakusei_blueprint (Math|Vector|Normalize (- (Transformation|GetWorldLocation (Variables|Default|GetStaticMeshComponent)) (Transformation|GetWorldLocation (Variables|/Script/Engine.StaticMeshActor|GetStaticMeshComponent _aswakusei_blueprint)))))) ; 移動ベクトルセット
          (Variables|/Game/Revive/Blueprints/MapObject/Wakusei_Blueprint.Wakusei_Blueprint_C|SetBHMove _aswakusei_blueprint (Math|Vector|MakeVector (.x _output_get) (.y _output_get) 0.0)) ; Z軸を０に
          (Variables|/Game/Revive/Blueprints/MapObject/Wakusei_Blueprint.Wakusei_Blueprint_C|SetLength _aswakusei_blueprint (Math|Vector|VectorLength (- (Transformation|GetWorldLocation (Variables|Default|GetStaticMeshComponent)) (Transformation|GetWorldLocation (Variables|/Script/Engine.StaticMeshActor|GetStaticMeshComponent _aswakusei_blueprint))))))
        (else
          (bind _outactors_2 (Actor|GetAllActorsOfClass "/Game/Revive/Blueprints/Character/ThirdPersonCharacter.ThirdPersonCharacter_C"))
          (for _array_element_2 _outactors_2
            (if (== _array_element_2 OtherActor) ; Playerかどうか
              (Variables|Default|SetBHPlayerSuikomiFlag true))))))))

(event OnComponentBeginOverlap(WarpCollision)
  (params (OverlappedComponent :type Primitive%20Component%20Object%20Reference) (OtherActor :type Actor%20Object%20Reference) (OtherComp :type Primitive%20Component%20Object%20Reference) (OtherBodyIndex :type Integer) (bFromSweep :type Boolean) (SweepResult :type Hit%20Result%20Structure%20%28by%20ref%29))
  ;[1 1 1] ワープ処理
  (if (Variables|Default|GetBHWHFlag)
    (bind _outactors (Actor|GetAllActorsOfClass "Wakusei_Child_Blackhole_BP_C"))
    (for _array_element _outactors
      (if (not (== _array_element OtherActor)) ; BHをはじく
        (if (Utilities|ClassIsChildOf (Utilities|GetClass OtherActor) "/Game/Revive/Blueprints/MapObject/Wakusei_Blueprint.Wakusei_Blueprint_C") ; 惑星かどうか
          (bind _aswakusei_blueprint (Utilities|Casting|CastToWakusei_Blueprint OtherActor))
          (if (Class|PrimitiveComponent|IsOverlappingComponent (Variables|Default|GetWarpCollision) (Variables|/Game/Revive/Blueprints/MapObject/Wakusei_Blueprint.Wakusei_Blueprint_C|GetSphere1 _aswakusei_blueprint))
            (Transformation|SetActorLocation OtherActor (Variables|Default|GetMyWhiteHole) false false)
            (Variables|/Game/Revive/Blueprints/MapObject/Wakusei_Blueprint.Wakusei_Blueprint_C|SetWhiteHoleFlag _aswakusei_blueprint true)
            (Variables|/Game/Revive/Blueprints/MapObject/Wakusei_Blueprint.Wakusei_Blueprint_C|SetBlackHoleFlag _aswakusei_blueprint false))
          (else
            (bind _outactors_2 (Actor|GetAllActorsOfClass "/Game/Revive/Blueprints/Character/ThirdPersonCharacter.ThirdPersonCharacter_C"))
            (for _array_element_2 _outactors_2
              (if (== _array_element_2 OtherActor) ; Playerかどうか
                (Variables|Default|SetBHPlayerSuikomiFlag false)
                (Variables|/Game/Revive/Blueprints/Character/ThirdPersonCharacter.ThirdPersonCharacter_C|SetWarpFlag _array_element_2 true)
                (Variables|Default|SetBHPlayerWarpFlag true)))))))))

(event EventBeginPlay
  (|CallParentFunction)
  (Rendering|SetVisibility (Variables|Default|GetBHparticle) false false) ; パーティクルセット
  (Components|Sphere|SetSphereRadius (Variables|Default|GetBlackHoleCollision) (Variables|Default|GetRadius) true) ; 吸い込み範囲セット
  (Variables|Default|SetMyWhiteHole (Transformation|GetWorldLocation (Variables|Default|GetWhiteHole))) ; WHの位置セット
)

(event Collision|EventActorBeginOverlap
  (params (OtherActor :type Actor%20Object%20Reference))
  (|CallParentFunction 0))

(event EventTick
  (params (DeltaSeconds :type Float%20%28single-precision%29))
  (bind _whradius (Variables|Default|GetWHRadius))
  (Utilities|FlowControl|Sequence
    (:then_0
      (if (Variables|Default|GetBHWHFlag) ; BHが生成されているか
        (Utilities|FlowControl|Sequence
          (:then_0
            (bind _outactors (Actor|GetAllActorsOfClass "/Game/Revive/Blueprints/MapObject/Wakusei_Blueprint.Wakusei_Blueprint_C"))
            (for _array_element _outactors
              (Utilities|FlowControl|Sequence
                (:then_0
                  ;[1 1 1] BH吸い込み処理
                  (if (Variables|/Game/Revive/Blueprints/MapObject/Wakusei_Blueprint.Wakusei_Blueprint_C|GetBlackHoleFlag _array_element) ; BHに吸われているか
                    (Transformation|AddActorWorldOffset _array_element (* (Variables|/Game/Revive/Blueprints/MapObject/Wakusei_Blueprint.Wakusei_Blueprint_C|GetBHMove _array_element) (+ (Variables|Default|GetBHsuikomiSpeed) (* (- 1.0 (/ (Math|Vector|VectorLength (- (Transformation|GetWorldLocation (Variables|Default|GetStaticMeshComponent)) (Transformation|GetWorldLocation (Variables|/Script/Engine.StaticMeshActor|GetStaticMeshComponent _array_element)))) (Variables|/Game/Revive/Blueprints/MapObject/Wakusei_Blueprint.Wakusei_Blueprint_C|GetLength _array_element))) 2e+01))))
                    (Development|PrintString (Utilities|String|ToString(Float) (/ (Math|Vector|VectorLength (- (Transformation|GetWorldLocation (Variables|Default|GetStaticMeshComponent)) (Transformation|GetWorldLocation (Variables|/Script/Engine.StaticMeshActor|GetStaticMeshComponent _array_element)))) (Variables|/Game/Revive/Blueprints/MapObject/Wakusei_Blueprint.Wakusei_Blueprint_C|GetLength _array_element))) true true "(R=0.000000,G=0.660000,B=1.000000,A=1.000000)" 0.0)))
                (:then_1
                  (if (Variables|/Game/Revive/Blueprints/MapObject/Wakusei_Blueprint.Wakusei_Blueprint_C|GetWhiteHoleFlag _array_element) ; WHに吐き出されているか
                    ;;[1 1 1] WH吐き出し終了処理
                    (if (<= (+ (.x (* (- (Variables|Default|GetMyWhiteHole) (Transformation|GetWorldLocation (Variables|/Script/Engine.StaticMeshActor|GetStaticMeshComponent _array_element))) (- (Variables|Default|GetMyWhiteHole) (Transformation|GetWorldLocation (Variables|/Script/Engine.StaticMeshActor|GetStaticMeshComponent _array_element))))) (.y (* (- (Variables|Default|GetMyWhiteHole) (Transformation|GetWorldLocation (Variables|/Script/Engine.StaticMeshActor|GetStaticMeshComponent _array_element))) (- (Variables|Default|GetMyWhiteHole) (Transformation|GetWorldLocation (Variables|/Script/Engine.StaticMeshActor|GetStaticMeshComponent _array_element)))))) (* _whradius _whradius)) ; WHの範囲に入っているか
                      (Transformation|AddActorWorldOffset _array_element (* (* (Variables|/Game/Revive/Blueprints/MapObject/Wakusei_Blueprint.Wakusei_Blueprint_C|GetBHMove _array_element) (+ (Variables|Default|GetBHsuikomiSpeed) (* (- 1.0 (/ (Math|Vector|VectorLength (- (Transformation|GetWorldLocation (Variables|Default|GetStaticMeshComponent)) (Transformation|GetWorldLocation (Variables|/Script/Engine.StaticMeshActor|GetStaticMeshComponent _array_element)))) (Variables|/Game/Revive/Blueprints/MapObject/Wakusei_Blueprint.Wakusei_Blueprint_C|GetLength _array_element))) 2e+01))) (- (/ (Math|Vector|VectorLength (- (Variables|Default|GetMyWhiteHole) (Transformation|GetWorldLocation (Variables|/Script/Engine.StaticMeshActor|GetStaticMeshComponent _array_element)))) (Variables|Default|GetWHRadius)) 1.0)))
                      (else
                        (Variables|/Game/Revive/Blueprints/MapObject/Wakusei_Blueprint.Wakusei_Blueprint_C|SetWhiteHoleFlag _array_element false))))))))
          (:then_1
            ;[1 1 1] Player吸い込み処理
            (if (Variables|Default|GetBHPlayerSuikomiFlag)
              (bind _outactors_2 (Actor|GetAllActorsOfClass "/Game/Revive/Blueprints/Character/ThirdPersonCharacter.ThirdPersonCharacter_C"))
              (for _array_element_2 _outactors_2
                (Transformation|AddActorWorldOffset _array_element_2 (* (Math|Vector|Normalize (- (Transformation|GetWorldLocation (Variables|Default|GetStaticMeshComponent)) (Transformation|GetWorldLocation (Variables|/Script/Engine.Actor|GetRootComponent _array_element_2)))) (Variables|Default|GetBHsuikomiSpeed))))))
          (:then_2
            ;[1 1 1] Playerワープ処理
            (if (Variables|Default|GetBHPlayerWarpFlag)
              (bind _outactors_3 (Actor|GetAllActorsOfClass "/Game/Revive/Blueprints/Character/ThirdPersonCharacter.ThirdPersonCharacter_C"))
              (for _array_element_3 _outactors_3
                (if (Variables|/Game/Revive/Blueprints/Character/ThirdPersonCharacter.ThirdPersonCharacter_C|GetWarpFlag _array_element_3)
                  (Transformation|AddActorWorldOffset _array_element_3 (* (- (Variables|Default|GetMyWhiteHole) (Transformation|GetWorldLocation (Variables|/Script/Engine.Actor|GetRootComponent _array_element_3))) 0.1))
                  (Variables|/Game/Revive/Blueprints/Character/ThirdPersonCharacter.ThirdPersonCharacter_C|SetFirstPosition _array_element_3 (Transformation|GetWorldLocation (Variables|/Script/Engine.Actor|GetRootComponent _array_element_3)))
                  (Rendering|SetVisibility (Variables|/Script/Engine.Character|GetMesh _array_element_3) false false)
                  (else
                    (Variables|Default|SetBHPlayerWarpFlag false)
                    (Rendering|SetVisibility (Variables|/Script/Engine.Character|GetMesh _array_element_3) true false))))))
          (:then_3
            ;[1 1 1] サイズ設定
            (Transformation|SetWorldScale3D (Variables|Default|GetBHparticle) "1.000000,1.000000,1.000000") ; BHのパーティクル大きさ設定
            (Transformation|SetWorldScale3D (Variables|Default|GetSphere1) "0, 0, 0") ; 実体の当たり判定消去
            (Transformation|SetWorldScale3D (Variables|Default|GetBlackHoleCollision) "1.000000,1.000000,1.000000") ; BHの大きさ固定(大きさ変える時はRadiusを変えて)
            (Transformation|SetWorldScale3D (Variables|Default|GetWarpCollision) "2.000000,2.000000,2.000000") ; BHの大きさ固定(大きさ変える時はRadiusを変えて)
          ))
        (else
          (|CallParentFunction DeltaSeconds)
          ;[1 1 1] HPが０になったらBH表示
          (if (<= (Variables|Default|GetP_HP) 0.0) ; HPが０になったらBH表示
            (Variables|Default|SetBHWHFlag true)
            (Rendering|SetVisibility (Variables|Default|GetBHparticle) true false)))))))

(fn ConstructionScript)