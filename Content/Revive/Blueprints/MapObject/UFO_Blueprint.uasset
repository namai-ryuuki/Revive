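; UFO map object that tracks an energy value (UHp) toward a maximum, starting at zero on play.
; Two camera-facing widget components show it as a gauge and number, refreshed every Tick.
; A sphere overlap notifies ThirdPersonCharacter via HitCallMessage and sets PlayerIn, which makes Tick add a new Suikomi_UI widget each frame.
; Once UHp reaches the maximum, Tick repeatedly sends CLEARBPIFMessage to OtherActor.
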(event OnComponentBeginOverlap(Sphere)
  (params (OverlappedComponent :type Primitive%20Component%20Object%20Reference) (OtherActor :type Actor%20Object%20Reference) (OtherComp :type Primitive%20Component%20Object%20Reference) (OtherBodyIndex :type Integer) (bFromSweep :type Boolean) (SweepResult :type Hit%20Result%20Structure%20%28by%20ref%29))
  ;[1 1 1] プレイヤーとの当たり判定（放出・吸収用）
  (if (== (Utilities|GetClass OtherActor) "/Game/Revive/Blueprints/Character/ThirdPersonCharacter.ThirdPersonCharacter_C")
    (Class|HITBPIF|HitCall(Message) OtherActor true)
    (Variables|Default|SetPlayer_In true)))

(event OnComponentEndOverlap(Sphere)
  (params (OverlappedComponent :type Primitive%20Component%20Object%20Reference) (OtherActor :type Actor%20Object%20Reference) (OtherComp :type Primitive%20Component%20Object%20Reference) (OtherBodyIndex :type Integer))
  ;[1 1 1] プレイヤーとの当たり判定（放出・吸収用）
  (if (== (Utilities|GetClass OtherActor) "/Game/Revive/Blueprints/Character/ThirdPersonCharacter.ThirdPersonCharacter_C")
    (Class|HITBPIF|HitCall(Message) OtherActor false)
    (Variables|Default|SetPlayer_In false)))

(event EventBeginPlay
  (bind _asenergie_ui (Utilities|Casting|CastToEnergie_UI (UserInterface|GetUserWidgetObject (Variables|Default|GetHP))))
  (bind _output_get (Variables|Default|SetHP_UI _asenergie_ui))
  (Variables|/Game/Revive/Blueprints/UI/Energie_UI.Energie_UI_C|SetEnergie _output_get 1.0)
  (bind _ashp_visible_ui (Utilities|Casting|CastToHP_Visible_UI (UserInterface|GetUserWidgetObject (Variables|Default|GetHP_Visibli))))
  (bind _output_get_2 (Variables|Default|SetHP_NUMBER _ashp_visible_ui))
  (Variables|/Game/Revive/Blueprints/UI/HP_Visible_UI.HP_Visible_UI_C|SetHP _output_get_2 (Variables|Default|GetU_MaxHp))
  (Variables|Default|SetU_Hp 0.0)
  (Variables|Default|SetU_MaxHp (Variables|Default|GetU_MaxHp)))

(event Collision|EventActorBeginOverlap
  (params (OtherActor :type Actor%20Object%20Reference)))

(event EventTick
  (params (DeltaSeconds :type Float%20%28single-precision%29))
  (Utilities|FlowControl|Sequence
    (:then_0
      ;[1 1 1] HPゲージが常にカメラを向くように設定
      (|CameraMove_2))
    (:then_1
      ;[1 1 1] HPの割合を求める
      (|HP＿WARIAI_2))
    (:then_2
      (if (<= (Variables|Default|GetU_MaxHp) (Variables|Default|GetU_Hp))
        (Class|ClearBPIF|CLEARBPIF(Message) (stale OnComponentBeginOverlap(Sphere) OtherActor))))
    (:then_3
      (if (Variables|Default|GetPlayer_In)
        (bind _returnvalue (UserInterface|CreateWidget "/Game/Revive/Blueprints/UI/Suikomi_UI.Suikomi_UI_C"))
        (UserInterface|Viewport|AddtoViewport _returnvalue 0)))))

(fn ConstructionScript)