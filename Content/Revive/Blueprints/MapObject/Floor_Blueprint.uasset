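; Floor actor Blueprint that builds a tiled floor in the map from a single static mesh.
; Its construction script runs nested loops over WidthCount and LengthCount, adding a static mesh component at each grid cell and assigning the StaticMesh variable.
; Tiles sit on a fixed 1000-unit spacing along X and Y from the actor origin.
; The event graph holds no active logic.
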(event EventBeginPlay)

(event Collision|EventActorBeginOverlap
  (params (OtherActor :type Actor%20Object%20Reference)))

(event EventTick
  (params (DeltaSeconds :type Float%20%28single-precision%29)))

(fn ConstructionScript
  (for _index (range 1 (Variables|Default|GetWidthCount)) ; 横幅のカウント
    (for _index_2 (range 1 (Variables|Default|GetLengthCount)) ; 縦幅のカウント
      (bind _returnvalue (AddComponent|AddStaticMeshComponent false (Math|Transform|MakeTransform (Math|Vector|MakeVector (* (- _index 1) 1e+03) (* (- _index_2 1) 1e+03) 0.0))))
      (Components|StaticMesh|SetStaticMesh _returnvalue (Variables|Default|GetStaticMesh)))))