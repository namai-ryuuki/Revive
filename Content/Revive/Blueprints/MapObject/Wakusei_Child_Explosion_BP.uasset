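; Explodable planet (Wakusei) map object that blows up when its HP runs out, hurting the player and nearby planets.
; Tick swaps material and toggles a particle at low HP, then on depletion spawns effects, shakes the camera and sets a tiny lifespan.
; Once dead, Bakuha overlap events, mainly EndOverlap, deliver damage and notify breakable walls.
; AnyDamage zeroes HP after a short delay, enabling chain explosions.
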(event OnComponentEndOverlap(bakuha)
  (params (OverlappedComponent :type Primitive%20Component%20Object%20Reference) (OtherActor :type Actor%20Object%20Reference) (OtherComp :type Primitive%20Component%20Object%20Reference) (OtherBodyIndex :type Integer))
  ;[1 1 1] 爆破したら範囲内のプレイヤーと惑星を爆破する
  (if (Variables|Default|Getdeath)
    (Utilities|FlowControl|Sequence
      (:then_0
        (if (== (Utilities|GetClass OtherActor) "/Game/Revive/Blueprints/Character/ThirdPersonCharacter.ThirdPersonCharacter_C")
          (Utilities|FlowControl|DoOnce false
            (:Completed
              (Class|WakuseiLocationBPIF|WakuseiLocation(Message) OtherActor (Transformation|GetWorldLocation (Variables|Default|GetStaticMeshComponent)))
              (Game|Damage|ApplyDamage OtherActor (Variables|Default|GetDamage) 0 0)))))
      (:then_1
        (if (Class|PrimitiveComponent|IsOverlappingComponent (Variables|Default|GetSphere) OtherComp)
          (Utilities|FlowControl|DoOnce false
            (:Completed
              (Game|Damage|ApplyDamage OtherActor 1.0 0 0)))))
      (:then_2
        (if (== (Utilities|GetClass OtherActor) "/Game/Revive/Blueprints/MapObject/BreakWall_BP.BreakWall_BP_C")
          (Utilities|FlowControl|DoOnce false
            (:Completed
              (Class|HITBPIF|HitCall(Message) OtherActor false))))))))

(event OnComponentBeginOverlap(bakuha)
  (params (OverlappedComponent :type Primitive%20Component%20Object%20Reference) (OtherActor :type Actor%20Object%20Reference) (OtherComp :type Primitive%20Component%20Object%20Reference) (OtherBodyIndex :type Integer) (bFromSweep :type Boolean) (SweepResult :type Hit%20Result%20Structure%20%28by%20ref%29))
  ;[1 1 1] 爆破したら範囲内のプレイヤーと惑星を爆破する
  (if (Variables|Default|Getdeath)
    (if (Class|PrimitiveComponent|IsOverlappingComponent (Variables|Default|GetSphere) OtherComp)
      (Game|Damage|ApplyDamage 0 1.0 0 0))))

(event EventBeginPlay
  (|CallParentFunction) ; This node is disabled and will not be called.\nDrag off pins to build functionality.
)

(event Collision|EventActorBeginOverlap
  (params (OtherActor :type Actor%20Object%20Reference))
  (|CallParentFunction OtherActor) ; This node is disabled and will not be called.\nDrag off pins to build functionality.
)

(event Game|Damage|EventAnyDamage
  (params (Damage :type Float%20%28single-precision%29) (DamageType :type Damage%20Type%20Object%20Reference) (InstigatedBy :type Controller%20Object%20Reference) (DamageCauser :type Actor%20Object%20Reference))
  (bind _returnvalue (Game|GetPlayerController 0))
  ;[1 1 1] 他の惑星の爆発に巻き込まれたら少し待って爆破する
  (Utilities|FlowControl|Delay 0.5)
  (Variables|Default|SetP_HP 0.0)
  (Variables|Default|SetP_TIME_MAXHP (Variables|Default|GetP_HP))
  (Class|PlayerCameraManager|PlayCameraShake (Variables|/Script/Engine.PlayerController|GetPlayerCameraManager _returnvalue) "/Game/Revive/Blueprints/MyCameraShake.MyCameraShake_C" 1.0 "CameraLocal" "0, 0, 0")
  (Game|Feedback|ClientPlayForceFeedback _returnvalue "/Game/Revive/Blueprints/NewForceFeedbackEffect.NewForceFeedbackEffect" false false "None"))

(event EventTick
  (params (DeltaSeconds :type Float%20%28single-precision%29))
  (bind _returnvalue (Game|GetPlayerController 0))
  (bind _particlesystem1 (Variables|Default|GetParticleSystem1))
  (|CallParentFunction DeltaSeconds)
  (Utilities|FlowControl|Sequence
    (:then_0
      ;[1 1 1] HPが0以下になったら爆発する
      (if (<= (Variables|Default|GetP_HP) 0.0)
        (Audio|PlaySoundatLocation "/Game/Revive/Sound/SE/se_explosion_Cue.se_explosion_Cue" (Transformation|GetActorLocation) "0, 0, 0" 1.0 1.0 0.0 "/Game/Revive/Sound/SE/se_explosionAttenuation.se_explosionAttenuation" 0 0)
        (Utilities|FlowControl|DoOnce false
          (:Completed
            (Effects|SpawnEmitteratLocation "/Game/InfinityBladeEffects/Effects/FX_Monsters/FX_Monster_Ausar/P_AU_ShieldSlam_AOE.P_AU_ShieldSlam_AOE" (Transformation|GetWorldLocation (Variables|Default|GetStaticMeshComponent)) "0, 0, 0" (* (Variables|Default|GetBakuhaHanni) 0.1))
            (Variables|Default|Setdeath true)
            (Actor|SetLifeSpan 0.02)
            (Class|PlayerCameraManager|PlayCameraShake (Variables|/Script/Engine.PlayerController|GetPlayerCameraManager _returnvalue) "/Game/Revive/Blueprints/MyCameraShake.MyCameraShake_C" 1.0 "CameraLocal" "0, 0, 0") ; カメラ振動
            (Game|Feedback|ClientPlayForceFeedback _returnvalue "/Game/Revive/Blueprints/NewForceFeedbackEffect.NewForceFeedbackEffect" false false "None")))))
    (:then_1
      ;[1 1 1] マテリアル変更
      (if (<= (Variables|/Game/Revive/Blueprints/UI/HP_UI.HP_UI_C|GetHP (Variables|Default|GetHP_UI)) 0.3)
        (if (>= (Variables|/Game/Revive/Blueprints/UI/HP_UI.HP_UI_C|GetHP (Variables|Default|GetHP_UI)) 0.15)
          (Rendering|Material|SetMaterial (Variables|Default|GetStaticMeshComponent) 0 "/DatasmithContent/Materials/CE_OpaqueMaster.CE_OpaqueMaster")
          (else
            (Rendering|Material|SetMaterial (Variables|Default|GetStaticMeshComponent) 0 "/DatasmithContent/Materials/FBXImporter/DeltaGenMasterTransparent.DeltaGenMasterTransparent")))
        (Transformation|SetWorldScale3D _particlesystem1 "2.000000,2.000000,2.000000")
        (Components|Activation|Activate _particlesystem1 false)
        (else
          (Rendering|Material|SetMaterial (Variables|Default|GetStaticMeshComponent) 0 "/Game/Revive/Material/BasicShapeMaterial.BasicShapeMaterial")
          (Components|Activation|Deactivate (Variables|Default|GetParticleSystem1)) ; パーティクル停止
        )))))

(fn ConstructionScript
  (|CallParentFunction))