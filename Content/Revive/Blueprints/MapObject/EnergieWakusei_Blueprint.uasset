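; Energy planet map actor whose HP sets its mesh size (capped) and drives camera-facing gauge and number widgets.
; An overlap sphere notifies the player for absorb/release, enabling particles and HP gain via WakuseiHpAdd.
; Tick also swaps material at low energy, shows ice/fire states from interface events, and orbits its start point while ZikuIn and player absent.
; Tick creates a new suction widget every frame the player is inside, unless frozen.
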(event OnComponentBeginOverlap(Sphere)
  (params (OverlappedComponent :type Primitive%20Component%20Object%20Reference) (OtherActor :type Actor%20Object%20Reference) (OtherComp :type Primitive%20Component%20Object%20Reference) (OtherBodyIndex :type Integer) (bFromSweep :type Boolean) (SweepResult :type Hit%20Result%20Structure%20%28by%20ref%29))
  ;[1 1 1] プレイヤーとの当たり判定（放出・吸収用）
  (if (== (Utilities|GetClass OtherActor) "/Game/Revive/Blueprints/Character/ThirdPersonCharacter.ThirdPersonCharacter_C")
    (Class|HITBPIF|HitCall(Message) OtherActor true)
    (if (not (Variables|Default|GetPlayer_In))
      (Variables|Default|SetPlayer_In true)
      (if (>= (Variables|Default|GetP_HP) 1e+01)
        (Variables|Default|SetP_TIMEHP (Variables|Default|GetP_HP))))))

(event OnComponentEndOverlap(Sphere)
  (params (OverlappedComponent :type Primitive%20Component%20Object%20Reference) (OtherActor :type Actor%20Object%20Reference) (OtherComp :type Primitive%20Component%20Object%20Reference) (OtherBodyIndex :type Integer))
  ;[1 1 1] プレイヤーとの当たり判定（放出・吸収用）
  (if (== (Utilities|GetClass OtherActor) "/Game/Revive/Blueprints/Character/ThirdPersonCharacter.ThirdPersonCharacter_C")
    (Class|HITBPIF|HitCall(Message) OtherActor false)
    (Variables|Default|SetPlayer_In false)))

(event EventBeginPlay
  ;[1 1 1] ウィジェット生成
  (bind _asenergie_ui (Utilities|Casting|CastToEnergie_UI (UserInterface|GetUserWidgetObject (Variables|Default|GetEnergie))))
  (bind _output_get (Variables|Default|SetEnergie_UI _asenergie_ui))
  (Variables|/Game/Revive/Blueprints/UI/Energie_UI.Energie_UI_C|SetEnergie _output_get 1.0)
  (bind _ashp_visible_ui (Utilities|Casting|CastToHP_Visible_UI (UserInterface|GetUserWidgetObject (Variables|Default|GetHP_Visibli))))
  (bind _output_get_2 (Variables|Default|SetHP_NUMBER _ashp_visible_ui))
  (Variables|/Game/Revive/Blueprints/UI/HP_Visible_UI.HP_Visible_UI_C|SetHP _output_get_2 (Variables|Default|GetP_MAXHP))
  (bind _output_get_3 (Variables|Default|SetP_HP (Variables|Default|GetP_MAXHP)))
  (Variables|Default|SetP_TIME_MAXHP _output_get_3)
  (Components|Activation|Deactivate (Variables|Default|GetParticleSystem)) ; パーティクル停止
  (Components|Activation|Deactivate (Variables|Default|GetParticleSystem1)) ; パーティクル停止
  (Variables|Default|SetStartPosition (Transformation|GetActorLocation))
  (Variables|Default|SetP_TIMEHP (Variables|Default|GetP_HP)))

(event EventTick
  (params (DeltaSeconds :type Float%20%28single-precision%29))
  (bind _p_hp (Variables|Default|GetP_HP))
  (bind _particlesystem1 (Variables|Default|GetParticleSystem1))
  (bind _returnvalue (* _p_hp 0.07))
  (bind _returnvalue_2 (Math|Float|Absolute(Float) _returnvalue))
  (Utilities|FlowControl|Sequence
    (:then_0
      ;[1 1 1] HPゲージが常にカメラを向くように設定
      (|CameraMove))
    (:then_1
      ;[1 1 1] HPの割合を求める
      (|HP＿WARIAI))
    (:then_2
      ;[1 1 1] パーティクルON/OFF
      (|Particle))
    (:then_3
      ;[1 1 1] 当たり判定の大きさ
      (if (> (Variables|Default|GetP_HP) 0.0)
        (bind _output_get (Variables|Default|Setscale_float _returnvalue_2))
        (if (>= _output_get 3.0)
          (Transformation|SetWorldScale3D (Variables|Debug|GetStaticMeshComponent) "3.000000,3.000000,3.000000") ; 大きさが3以上だったら３にする
          (Transformation|SetWorldScale3D (Variables|Default|GetSphere) "10.000000,10.000000,10.000000")
          (Transformation|SetWorldScale3D (Variables|Default|GetSphere1) "7.000000,8.000000,8.000000")
          (Transformation|SetWorldScale3D (Variables|Default|Getbakuha) (Variables|Default|GetBakuhaHanni))
          (Transformation|SetWorldScale3D (Variables|Default|GetEnergie) "2.500000,2.500000,2.500000")
          (else
            (Transformation|SetWorldScale3D (Variables|Debug|GetStaticMeshComponent) (Math|Conversions|ToVector(Float) _returnvalue_2))))))
    (:then_4
      ;[1 1 1] 凍る見た目処理
      (if (Variables|Default|GetIceFlag)
        (Rendering|SetVisibility (Variables|Default|Getice) true false)
        (else
          (Rendering|SetVisibility (Variables|Default|Getice) false false))))
    (:then_5
      ;[1 1 1] パーティクル
      (if (<= (Variables|/Game/Revive/Blueprints/UI/Energie_UI.Energie_UI_C|GetEnergie (Variables|Default|GetEnergie_UI)) 0.3)
        (if (>= (Variables|/Game/Revive/Blueprints/UI/Energie_UI.Energie_UI_C|GetEnergie (Variables|Default|GetEnergie_UI)) 0.15)
          (Rendering|Material|SetMaterial (Variables|Debug|GetStaticMeshComponent) 0 "/DatasmithContent/Materials/CE_OpaqueMaster.CE_OpaqueMaster")
          (else
            (Rendering|Material|SetMaterial (Variables|Debug|GetStaticMeshComponent) 0 "/DatasmithContent/Materials/FBXImporter/DeltaGenMasterTransparent.DeltaGenMasterTransparent")))
        (Transformation|SetWorldScale3D _particlesystem1 "2.000000,2.000000,2.000000")
        (Components|Activation|Activate _particlesystem1 false)
        (else
          (Components|Activation|Deactivate (Variables|Default|GetParticleSystem1)) ; パーティクル停止
        )))
    (:then_6
      ;[1 1 1] 星の回転
      (if (Math|Boolean|NotEqual(Boolean) (Variables|Default|GetPlayer_In) true) ; プレイヤーに接触してたら止まる
        (if (Variables|Default|GetZiku_In)
          (Transformation|AddActorLocalRotation (Variables|Default|GetRotationStarSpeed) false false)
          (bind _output_get_2 (Variables|Default|SetDirectionVector (Math|Rotator|GetRotationXVector (Transformation|GetActorRotation))))
          (Transformation|SetActorLocation (+ (Variables|Default|GetStartPosition) (* (Math|Vector|Normalize _output_get_2) (Variables|Default|GetDistance))) false false)
          (Development|PrintString (Utilities|String|ToString(Vector) (Variables|Default|GetRotationMove)) true true "(R=0.000000,G=0.660000,B=1.000000,A=1.000000)" 0.0))))
    (:then_7
      ;[1 1 1] 吸い込みUI
      (if (Variables|Default|GetPlayer_In)
        (if (not (Variables|Default|GetIceFlag))
          (bind _returnvalue_3 (UserInterface|CreateWidget "/Game/Revive/Blueprints/UI/Suikomi_UI.Suikomi_UI_C"))
          (UserInterface|Viewport|AddtoViewport _returnvalue_3 0))))
    (:then_8
      ;[1 1 1] 太陽で氷を溶かす処理
      (if (not (Variables|Default|GetIceFlag))
        (if (Variables|Default|GetFireFlag)
          (Components|Activation|Activate (Variables|Default|GetP_Spinner_Arm_Fire) false) ; パーティクル再生
          (else
            (Components|Activation|Deactivate (Variables|Default|GetP_Spinner_Arm_Fire)) ; パーティクル停止
          ))))))

(event EventWakuseiHpAdd
  ;[1 1 1] HPを与える処理
  (if (Variables|Default|GetPlayer_In)
    (if (>= (Variables|Default|GetP_MAXHP) (Variables|Default|GetP_HP))
      (bind _output_get (Variables|Default|SetP_HP (+ (Variables|Default|GetP_HP) (Variables|Default|Gethp_add))))
      (Variables|Default|SetP_TIME_MAXHP _output_get))))

(event EventZikuHanni
  (params (flag :type Boolean) (location :type Vector :default "0, 0, 0") (Component :type Static%20Mesh%20Component%20Object%20Reference))
  ;[1 1 1] 軸イベント
  (Variables|Default|SetZiku_In flag)
  (Variables|Default|SetRotationMove location))

(event Collision|EventActorBeginOverlap
  (params (OtherActor :type Actor%20Object%20Reference)))

(event EventFireBPIF
  (params (flag :type Boolean))
  ;[1 1 1] BPIF取得
  (Variables|Default|SetFireFlag flag))

(event EventICEBPIF
  (params (flag :type Boolean))
  ;[1 1 1] BPIF取得
  (Variables|Default|SetIceFlag flag))

(fn ConstructionScript
  (bind _p_maxhp (Variables|Default|GetP_MAXHP))
  (bind _staticmeshcomponent (Variables|Debug|GetStaticMeshComponent))
  (bind _returnvalue (* _p_maxhp 0.07))
  (bind _returnvalue_2 (Math|Float|Absolute(Float) _returnvalue))
  (Transformation|SetWorldScale3D (Variables|Default|Getbakuha) (Variables|Default|GetBakuhaHanni))
  (bind _output_get (Variables|Default|Setscale_float _returnvalue_2))
  (if (>= _output_get 3.0)
    (Transformation|SetWorldScale3D _staticmeshcomponent "3.000000,3.000000,3.000000") ; 大きさが3以上だったら３にする
    (else
      (Transformation|SetWorldScale3D _staticmeshcomponent (Math|Conversions|ToVector(Float) _returnvalue_2))))
  (Transformation|SetWorldScale3D (Variables|Default|GetSphere) "10.000000,10.000000,10.000000")
  (Transformation|SetWorldScale3D (Variables|Default|GetSphere1) "7.000000,8.000000,8.000000")
  (Rendering|SetVisibility (Variables|Default|GetSphere1) false false))