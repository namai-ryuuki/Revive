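; Exploding planet actor that respawns a copy of itself when its HP UI empties, making it an endless planet.
; Tick swaps materials and starts particles at low HP, and at zero PHP plays blast effects, camera shake and rumble before expiring.
; Once dead, Bakuha overlaps damage the player and other non-Infinite actors.
; Any incoming damage zeroes PHP after a short delay, so neighbouring blasts can set it off.
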(event OnComponentEndOverlap(bakuha)
  (params (OverlappedComponent :type Primitive%20Component%20Object%20Reference) (OtherActor :type Actor%20Object%20Reference) (OtherComp :type Primitive%20Component%20Object%20Reference) (OtherBodyIndex :type Integer))
  ;[1 1 1] 爆破したら範囲内のプレイヤーと惑星を爆破する
  (if (Variables|Default|Getdeath)
    (if (== (Utilities|GetClass OtherActor) "/Game/Revive/Blueprints/Character/ThirdPersonCharacter.ThirdPersonCharacter_C")
      (Utilities|FlowControl|DoOnce false
        (:Completed
          (Class|WakuseiLocationBPIF|WakuseiLocation(Message) OtherActor (Transformation|GetWorldLocation (Variables|Default|GetStaticMeshComponent)))
          (Game|Damage|ApplyDamage OtherActor (Variables|Default|GetDamage) 0 0)))
      (elif (Class|PrimitiveComponent|IsOverlappingComponent (Variables|Default|GetSphere) OtherComp)
        (if (!= (Utilities|GetClass OtherActor) "Wakusei_Infinite_BP_C")
          (Game|Damage|ApplyDamage OtherActor 1.0 0 0))))))

(event OnComponentBeginOverlap(bakuha)
  (params (OverlappedComponent :type Primitive%20Component%20Object%20Reference) (OtherActor :type Actor%20Object%20Reference) (OtherComp :type Primitive%20Component%20Object%20Reference) (OtherBodyIndex :type Integer) (bFromSweep :type Boolean) (SweepResult :type Hit%20Result%20Structure%20%28by%20ref%29))
  ;[1 1 1] 爆破したら範囲内のプレイヤーと惑星を爆破する
  (if (Variables|Default|Getdeath)
    (if (Class|PrimitiveComponent|IsOverlappingComponent (Variables|Default|GetSphere) OtherComp)
      (if (!= (Utilities|GetClass OtherActor) "Wakusei_Infinite_BP_C")
        (Game|Damage|ApplyDamage OtherActor 1.0 0 0)))))

(event EventBeginPlay
  (bind _p_hp (Variables|Default|GetP_HP))
  (|CallParentFunction)
  (Variables|Default|SetP_MAXHP _p_hp)
  (bind _output_get (Variables|Default|SetP_TIME_MAXHP _p_hp))
  (Variables|Default|SetP_TIMEHP _output_get))

(event Collision|EventActorBeginOverlap
  (params (OtherActor :type Actor%20Object%20Reference))
  (|CallParentFunction OtherActor) ; This node is disabled and will not be called.\nDrag off pins to build functionality.
)

(event Game|Damage|EventAnyDamage
  (params (Damage :type Float%20%28single-precision%29) (DamageType :type Damage%20Type%20Object%20Reference) (InstigatedBy :type Controller%20Object%20Reference) (DamageCauser :type Actor%20Object%20Reference))
  (bind _returnvalue (Game|GetPlayerController 0))
  ;[1 1 1] 他の惑星の爆発に巻き込まれたら少し待って爆破する
  (Utilities|FlowControl|Delay 0.5)
  (Variables|Default|SetP_HP 0.0)
  (Variables|Default|SetP_TIME_MAXHP (Variables|Default|GetP_HP))
  (Class|PlayerCameraManager|PlayCameraShake (Variables|/Script/Engine.PlayerController|GetPlayerCameraManager _returnvalue) "/Game/Revive/Blueprints/MyCameraShake.MyCameraShake_C" 1.0 "CameraLocal" "0, 0, 0")
  (Game|Feedback|ClientPlayForceFeedback _returnvalue "/Game/Revive/Blueprints/NewForceFeedbackEffect.NewForceFeedbackEffect" false false "None"))

(event EventTick
  (params (DeltaSeconds :type Float%20%28single-precision%29))
  (bind _returnvalue (Game|GetPlayerController 0))
  (bind _particlesystem1 (Variables|Default|GetParticleSystem1))
  (|CallParentFunction DeltaSeconds)
  (Utilities|FlowControl|Sequence
    (:then_0
      ;[1 1 1] HPが0以下になったら爆発する
      (if (<= (Variables|Default|GetP_HP) 0.0)
        (Audio|PlaySoundatLocation "/Game/Revive/Sound/SE/se_explosion_Cue.se_explosion_Cue" (Transformation|GetActorLocation) "0, 0, 0" 1.0 1.0 0.0 "/Game/Revive/Sound/SE/se_explosionAttenuation.se_explosionAttenuation" 0 0)
        (Utilities|FlowControl|DoOnce false
          (:Completed
            (Effects|SpawnEmitteratLocation "/Game/InfinityBladeEffects/Effects/FX_Monsters/FX_Monster_Ausar/P_AU_ShieldSlam_AOE.P_AU_ShieldSlam_AOE" (Transformation|GetWorldLocation (Variables|Default|GetStaticMeshComponent)) "0, 0, 0" (* (Variables|Default|GetBakuhaHanni) 0.1))
            (Variables|Default|Setdeath true)
            (Actor|SetLifeSpan 0.5)
            (Class|PlayerCameraManager|PlayCameraShake (Variables|/Script/Engine.PlayerController|GetPlayerCameraManager _returnvalue) "/Game/Revive/Blueprints/MyCameraShake.MyCameraShake_C" 1.0 "CameraLocal" "0, 0, 0") ; カメラ振動
            (Game|Feedback|ClientPlayForceFeedback _returnvalue "/Game/Revive/Blueprints/NewForceFeedbackEffect.NewForceFeedbackEffect" false false "None")))))
    (:then_1
      ;[1 1 1] マテリアル変更
      (if (<= (Variables|/Game/Revive/Blueprints/UI/HP_UI.HP_UI_C|GetHP (Variables|Default|GetHP_UI)) 0.3)
        (if (>= (Variables|/Game/Revive/Blueprints/UI/HP_UI.HP_UI_C|GetHP (Variables|Default|GetHP_UI)) 0.15)
          (Rendering|Material|SetMaterial (Variables|Default|GetStaticMeshComponent) 0 "/DatasmithContent/Materials/CE_OpaqueMaster.CE_OpaqueMaster")
          (else
            (Rendering|Material|SetMaterial (Variables|Default|GetStaticMeshComponent) 0 "/DatasmithContent/Materials/FBXImporter/DeltaGenMasterTransparent.DeltaGenMasterTransparent")))
        (Transformation|SetWorldScale3D _particlesystem1 "2.000000,2.000000,2.000000")
        (Components|Activation|Activate _particlesystem1 false)
        (else
          (Components|Activation|Deactivate (Variables|Default|GetParticleSystem1)) ; パーティクル停止
        )))
    (:then_2
      ;[1 1 1] 星の復活
      (if (<= (Variables|/Game/Revive/Blueprints/UI/HP_UI.HP_UI_C|GetHP (Variables|Default|GetHP_UI)) 0.0)
        (Utilities|FlowControl|DoOnce false
          (:Completed
            (Game|SpawnActorfromClass "Wakusei_Infinite_BP_C" (Transformation|GetWorldTransform (Variables|Default|GetStaticMeshComponent)) "Undefined" 0 1e+01 "20.000000,20.000000,20.000000" 0 1e+01)
            ;;[1 1 1] プレイヤーのHPを減らす減点を今の場所に！
            (bind _asthird_person_character (Utilities|Casting|CastToThirdPersonCharacter (Game|GetPlayerCharacter 0)))
            (Variables|Default|SetP_HP (Variables|/Game/Revive/Blueprints/Character/ThirdPersonCharacter.ThirdPersonCharacter_C|GetP_HP _asthird_person_character))
            (Variables|/Game/Revive/Blueprints/Character/ThirdPersonCharacter.ThirdPersonCharacter_C|SetFirstPosition _asthird_person_character (Transformation|GetWorldLocation (Variables|/Script/Engine.Character|GetCapsuleComponent _asthird_person_character)))))))))

(fn ConstructionScript
  (|CallParentFunction))