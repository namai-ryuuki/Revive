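; Ice planet map object, a child Blueprint that shares its HP with nearby planets and changes appearance when depleted.
; Each Tick it scales the Bakuha (blast) range by half its HP and writes that HP to IceGetHp on normal and energy planets overlapping Sphere2, found through GetAllActorsOfClass.
; It zeroes IceGetHp on the end-overlap actor once clear of Sphere.
; Positive HP activates ice particles; otherwise they stop and the Delice component shows.
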(event OnComponentEndOverlap(Sphere)
  (params (OverlappedComponent :type Primitive%20Component%20Object%20Reference) (OtherActor :type Actor%20Object%20Reference) (OtherComp :type Primitive%20Component%20Object%20Reference) (OtherBodyIndex :type Integer))
  ;[1 1 1] COLLISION
)

(event EventBeginPlay
  ;[1 1 1] BEGIN
  (|CallParentFunction))

(event Collision|EventActorBeginOverlap
  (params (OtherActor :type Actor%20Object%20Reference))
  (|CallParentFunction OtherActor) ; This node is disabled and will not be called.\nDrag off pins to build functionality.
)

(event EventTick
  (params (DeltaSeconds :type Float%20%28single-precision%29))
  (bind _iceplanet (Variables|Default|Geticeplanet))
  (bind _delice (Variables|Default|Getdelice))
  (bind _staticmeshcomponent (Variables|Default|GetStaticMeshComponent))
  ;[1 1 1] UPDATE
  (|CallParentFunction DeltaSeconds)
  (Utilities|FlowControl|Sequence
    (:then_0
      (bind _output_get (Variables|Default|SetBakuhaHanni (Math|Conversions|ToVector(Float) (* (Variables|Default|GetP_HP) 0.5))))
      (Transformation|SetWorldScale3D (Variables|Default|Getbakuha) _output_get)
      (Rendering|SetVisibility (Variables|Default|Getdelice) false false))
    (:then_1
      (Variables|Default|SetFireFlag false)
      (Variables|Default|SetIceFlag false))
    (:then_2
      (bind _outactors (Actor|GetAllActorsOfClass "/Game/Revive/Blueprints/MapObject/Wakusei_Blueprint.Wakusei_Blueprint_C"))
      (for _array_element _outactors
        (bind _aswakusei_blueprint (Utilities|Casting|CastToWakusei_Blueprint _array_element))
        (if (Class|PrimitiveComponent|IsOverlappingComponent (Variables|Default|GetSphere2) (Variables|/Game/Revive/Blueprints/MapObject/Wakusei_Blueprint.Wakusei_Blueprint_C|GetSphere _aswakusei_blueprint))
          (Variables|/Game/Revive/Blueprints/MapObject/Wakusei_Blueprint.Wakusei_Blueprint_C|SetIceGetHp _aswakusei_blueprint (Variables|Default|GetP_HP)))))
    (:then_3
      (bind _outactors_2 (Actor|GetAllActorsOfClass "/Game/Revive/Blueprints/MapObject/EnergieWakusei_Blueprint.EnergieWakusei_Blueprint_C"))
      (for _array_element_2 _outactors_2
        (bind _asenergie_wakusei_blueprint (Utilities|Casting|CastToEnergieWakusei_Blueprint _array_element_2))
        (if (Class|PrimitiveComponent|IsOverlappingComponent (Variables|Default|GetSphere2) (Variables|/Game/Revive/Blueprints/MapObject/EnergieWakusei_Blueprint.EnergieWakusei_Blueprint_C|GetSphere _asenergie_wakusei_blueprint))
          (Variables|/Game/Revive/Blueprints/MapObject/EnergieWakusei_Blueprint.EnergieWakusei_Blueprint_C|SetIceGetHp _asenergie_wakusei_blueprint (Variables|Default|GetP_HP)))))
    (:then_4
      ;[1 1 1] COLLISION
      (Utilities|FlowControl|Sequence
        (:then_0
          ;;[1 1 1] wakuseiがIceWakuseiと当たっていなかったらWakuseiの体力に０を代入する
          (if (Utilities|ClassIsChildOf (Utilities|GetClass (stale OnComponentEndOverlap(Sphere) OtherActor)) "/Game/Revive/Blueprints/MapObject/Wakusei_Blueprint.Wakusei_Blueprint_C")
            (bind _aswakusei_blueprint_2 (Utilities|Casting|CastToWakusei_Blueprint (stale OnComponentEndOverlap(Sphere) OtherActor)))
            (if (not (Class|PrimitiveComponent|IsOverlappingComponent (Variables|Default|GetSphere) (Variables|/Game/Revive/Blueprints/MapObject/Wakusei_Blueprint.Wakusei_Blueprint_C|GetSphere _aswakusei_blueprint_2)))
              (Variables|/Game/Revive/Blueprints/MapObject/Wakusei_Blueprint.Wakusei_Blueprint_C|SetIceGetHp _aswakusei_blueprint_2 0.0))))
        (:then_1
          ;;[1 1 1] EnergiewakuseiがIceWakuseiと当たっていなかったらEnergieWakuseiの体力に０を代入する
          (if (Utilities|ClassIsChildOf (Utilities|GetClass (stale OnComponentEndOverlap(Sphere) OtherActor)) "/Game/Revive/Blueprints/MapObject/EnergieWakusei_Blueprint.EnergieWakusei_Blueprint_C")
            (bind _asenergie_wakusei_blueprint_2 (Utilities|Casting|CastToEnergieWakusei_Blueprint (stale OnComponentEndOverlap(Sphere) OtherActor)))
            (if (not (Class|PrimitiveComponent|IsOverlappingComponent (Variables|Default|GetSphere) (Variables|/Game/Revive/Blueprints/MapObject/EnergieWakusei_Blueprint.EnergieWakusei_Blueprint_C|GetSphere _asenergie_wakusei_blueprint_2)))
              (Variables|/Game/Revive/Blueprints/MapObject/EnergieWakusei_Blueprint.EnergieWakusei_Blueprint_C|SetIceGetHp _asenergie_wakusei_blueprint_2 0.0))))))
    (:then_5
      (Transformation|SetWorldScale3D (Variables|Default|GetStaticMeshComponent) "4.000000,4.000000,4.000000")
      (Transformation|SetWorldScale3D (Variables|Default|GetHP) "2.500000,2.500000,2.500000"))
    (:then_6
      (if (> (Variables|Default|GetP_HP) 0.0)
        (Components|Activation|Activate _iceplanet false) ; パーティクル再生
        (Rendering|SetVisibility _delice false false)
        (Rendering|SetVisibility _staticmeshcomponent false false)
        (else
          (Components|Activation|Deactivate _iceplanet) ; パーティクル停止
          (Rendering|SetVisibility _staticmeshcomponent false false)
          (Rendering|SetVisibility _delice true false))))))

(fn ConstructionScript
  (|CallParentFunction))