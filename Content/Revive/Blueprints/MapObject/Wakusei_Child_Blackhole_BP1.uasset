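; Black hole map object that pulls in overlapping actors and warps qualifying ones to a white hole.
; Entering BlackHoleCollision starts a timeline that eases the actor toward the hole's mesh.
; Actor overlap caches the location of the last actor found by a class search as the white-hole point.
; The warp collision checks class and component overlap, then teleports the actor to a random point in a box there.
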(event OnComponentBeginOverlap(BlackHoleCollision)
  (params (OverlappedComponent :type Primitive%20Component%20Object%20Reference) (OtherActor :type Actor%20Object%20Reference) (OtherComp :type Primitive%20Component%20Object%20Reference) (OtherBodyIndex :type Integer) (bFromSweep :type Boolean) (SweepResult :type Hit%20Result%20Structure%20%28by%20ref%29))
  (bind _新規track_0 (Timeline|タイムライン_0 Play)
    (:Update
      (Transformation|SetActorLocation OtherActor (Math|Interpolation|Ease "EaseInOut" (/ _新規track_0 1e+01) (Transformation|GetActorLocation OtherActor) (Transformation|GetWorldLocation (Variables|Default|GetStaticMeshComponent)) 1.0) false false))))

(event OnComponentBeginOverlap(WarpCollision_0)
  (params (OverlappedComponent :type Primitive%20Component%20Object%20Reference) (OtherActor :type Actor%20Object%20Reference) (OtherComp :type Primitive%20Component%20Object%20Reference) (OtherBodyIndex :type Integer) (bFromSweep :type Boolean) (SweepResult :type Hit%20Result%20Structure%20%28by%20ref%29))
  (if (Utilities|ClassIsChildOf (Utilities|GetClass OtherActor) 0)
    (bind _aswakusei_blueprint (Utilities|Casting|CastTo OtherActor))
    (if (Class|PrimitiveComponent|IsOverlappingComponent (Variables|Default|GetWarpCollision_0) (Variables|Default|GetWarpCollision _aswakusei_blueprint))
      (Transformation|SetActorLocation OtherActor (Math|Random|RandomPointinBoundingBox (Variables|Default|Getmywhiteholl) (Variables|Default|Getbighall)) false false)
      (Development|PrintString "hit"))))

(event EventBeginPlay)

(event Collision|EventActorBeginOverlap
  (params (OtherActor :type Actor%20Object%20Reference))
  (bind _outactors (Actor|GetAllActorsOfClass 0))
  (for _array_element _outactors
    (Variables|Default|Setmywhiteholl (Transformation|GetWorldLocation (Variables|/Script/Engine.StaticMeshActor|GetStaticMeshComponent _array_element)))))

(event EventTick
  (params (DeltaSeconds :type Float%20%28single-precision%29)))

(fn ConstructionScript)