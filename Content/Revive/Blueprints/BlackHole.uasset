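; BlackHole is an actor that pulls in overlapping actors and teleports them to a white hole.
; Overlapping its sphere, enlarged at BeginPlay, starts a timeline that eases the other actor from its current location toward the black hole's mesh.
; When finished, the actor jumps to a random point in a box around the stored white hole position.
; Actor overlap refreshes that position from the last WhiteHall actor found.
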(event OnComponentBeginOverlap(Sphere_Collision)
  (params (OverlappedComponent :type Primitive%20Component%20Object%20Reference) (OtherActor :type Actor%20Object%20Reference) (OtherComp :type Primitive%20Component%20Object%20Reference) (OtherBodyIndex :type Integer) (bFromSweep :type Boolean) (SweepResult :type Hit%20Result%20Structure%20%28by%20ref%29))
  (bind _新規track_0 (Timeline|タイムライン_0 PlayFromStart)
    (:Update
      (Transformation|SetActorLocation OtherActor (Math|Interpolation|Ease "EaseInOut" _新規track_0 (Transformation|GetActorLocation OtherActor) (Transformation|GetWorldLocation (Variables|Debug|GetStaticMeshComponent)) 1.0) false false))
    (:Finished
      (Transformation|SetActorLocation OtherActor (Math|Random|RandomPointinBoundingBox (Variables|Default|Getmywhiteholl) (Variables|Default|Getbighall)) false false)
      (Development|PrintString "hit"))))

(event EventBeginPlay
  (Transformation|SetWorldScale3D (Variables|Default|GetSphere_Collision) "5.000000,5.000000,5.000000"))

(event Collision|EventActorBeginOverlap
  (params (OtherActor :type Actor%20Object%20Reference))
  (bind _outactors (Actor|GetAllActorsOfClass "/Game/ThirdPersonBP/Blueprints/WhiteHall.WhiteHall_C"))
  (for _array_element _outactors
    (Variables|Default|Setmywhiteholl (Transformation|GetWorldLocation (Variables|/Script/Engine.StaticMeshActor|GetStaticMeshComponent _array_element)))))

(fn ConstructionScript)