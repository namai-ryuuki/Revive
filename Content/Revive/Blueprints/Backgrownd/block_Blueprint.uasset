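; Background block Blueprint that builds a grid of static mesh tiles in its construction script, with no active gameplay logic.
; Nested width and length loops add one mesh component per cell at fixed spacing, all using the configurable mesh.
; A running counter alternates each successive block between no rotation and a slight tilt on all three axes.
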(event EventBeginPlay)

(event Collision|EventActorBeginOverlap
  (params (OtherActor :type Actor%20Object%20Reference)))

(event EventTick
  (params (DeltaSeconds :type Float%20%28single-precision%29)))

(fn ConstructionScript
  (for _index (range 1 (Variables|Default|GetWidthCount)) ; 横幅のカウント
    (for _index_2 (range 1 (Variables|Default|GetLengthCount)) ; 縦幅のカウント
      (if (<= (Math|Integer|%(Integer) (Variables|Default|Getfor_index) 2) 0)
        (Variables|Default|SetRotation "0, 0, 0")
        (else
          (Variables|Default|SetRotation "22.000000,22.000000,22.000000")))
      (bind _returnvalue (AddComponent|AddStaticMeshComponent false (Math|Transform|MakeTransform (Math|Vector|MakeVector (* (- _index 1) 1e+02) (* (- _index_2 1) 1e+02) 0.0) (Variables|Default|GetRotation))))
      (bind _output_get (Variables|Default|Setfor_index (+ (Variables|Default|Getfor_index) 1)))
      (Components|StaticMesh|SetStaticMesh _returnvalue (Variables|Default|GetStaticMesh)))))